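; BP_Potion_01 is a potion pickup actor that shows an interaction prompt when something overlaps its sphere.
; On BeginPlay it creates a hidden WBP_Interact widget, and sphere overlaps toggle both its visibility and the IsClose flag, without filtering the overlapping actor.
; The Take_Potion event hides the prompt and destroys the actor if IsClose is set, with no potion effect applied here.
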(event OnComponentBeginOverlap(Sphere)
  (params (OverlappedComponent :type Primitive%20Component%20Object%20Reference) (OtherActor :type Actor%20Object%20Reference) (OtherComp :type Primitive%20Component%20Object%20Reference) (OtherBodyIndex :type Integer) (bFromSweep :type Boolean) (SweepResult :type Hit%20Result%20Structure%20%28by%20ref%29))
  (Variables|Default|Setis_close true)
  (Variables|/Script/UMG.Widget|SetVisibility (stale EventBeginPlay _returnvalue) "Visible"))

(event OnComponentEndOverlap(Sphere)
  (params (OverlappedComponent :type Primitive%20Component%20Object%20Reference) (OtherActor :type Actor%20Object%20Reference) (OtherComp :type Primitive%20Component%20Object%20Reference) (OtherBodyIndex :type Integer))
  (Variables|Default|Setis_close false)
  (Variables|/Script/UMG.Widget|SetVisibility (stale EventBeginPlay _returnvalue) "Hidden"))

(event Custom|Take_Potion
  (if (Variables|Default|Getis_close)
    (Variables|/Script/UMG.Widget|SetVisibility (stale EventBeginPlay _returnvalue) "Hidden")
    (Actor|DestroyActor)))

(event EventBeginPlay
  (bind _returnvalue (UserInterface|CreateWidget "/Game/Assets/ui/WBP_Interact.WBP_Interact_C"))
  (UserInterface|Viewport|AddtoViewport _returnvalue 0)
  (Variables|/Script/UMG.Widget|SetVisibility _returnvalue "Hidden"))

(event Collision|EventActorBeginOverlap
  (params (OtherActor :type Actor%20Object%20Reference)))

(event EventTick
  (params (DeltaSeconds :type Float%20%28single-precision%29)))

(fn ConstructionScript)